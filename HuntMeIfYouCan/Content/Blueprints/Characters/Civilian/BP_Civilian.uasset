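; Civilian character Blueprint that runs server-side NPC wandering, despawning and respawning.
; BeginPlay randomly starts the NPC either walking or idle with a randomized lifetime before despawn.
; Tick uses the IsWalkFinished flag and random delays to repeat AIMoveTo to random nearby navigable points.
; Death or lifetime expiry stops movement and destroys the actor after a short delay, and Destroyed calls CivilianRespawn.
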(event `self.ReceiveBeginPlay`
  (`KismetSystemLibrary.Delay` 0.5)
  (`/Engine/EditorBlueprintResources/ActorMacros.Switch Has Authority`
    (:`Authority`
      (if (`self.bIsNPC`)
        (bind _output_get (set `self.bIsWalkFinished` (`KismetMathLibrary.RandomBool`)))
        (if _output_get
          (if (`self.bIsNPC`)
            (`KismetSystemLibrary.Delay` (`KismetMathLibrary.RandomFloatInRange` 60.0 90.0))
            (`MovementComponent.StopMovementImmediately` (`self.CharacterMovement`) :!label _label)
            (`KismetSystemLibrary.Delay` 3.0)
            (`self.K2_DestroyActor`))
          (else
            (`/Engine/EditorBlueprintResources/StandardMacros.DoOnce` false
              (:`Completed`
                (`|AIMoveTo` self (`NavigationSystem.GetRandomPointInNavigableRadius` (`self.K2_GetActorLocation`) 1000.0) null 5.0 true :!label _label_2
                  (:`then`
                    (set `self.bIsWalkFinished` true)))))))))))

(event `self.ReceiveActorBeginOverlap`
  (params (OtherActor :type "Actor Object Reference")))

(event `self.ReceiveTick`
  (params (DeltaSeconds :type "Float (single-precision)"))
  (`/Engine/EditorBlueprintResources/ActorMacros.Switch Has Authority`
    (:`Authority`
      (if (`self.bIsNPC`)
        (if (`self.bIsDead`)
          (goto _label)
          (elif (`self.bIsWalkFinished`)
            (set `self.bIsWalkFinished` false)
            (`KismetSystemLibrary.Delay` (`KismetMathLibrary.RandomFloatInRange` 6.5 10.0))
            (if (`self.bIsDead`)
              (goto _label)
              (else
                (goto _label_2)))))))))

(event `self.ReceiveDestroyed`
  (`/Engine/EditorBlueprintResources/ActorMacros.Switch Has Authority`
    (:`Authority`
      (`SpawnerFunctionLibrary.CivilianRespawn`)
      (`self.SetLifeSpan` 0.0))))

(fn `UserConstructionScript`)