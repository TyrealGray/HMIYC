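; BP_HMIYCGameInstance is the game instance that handles hosting, joining and leaving multiplayer sessions through three custom events.
; Hosting creates a LAN session for the first player controller and, on success, opens the WestTown map as a listen server.
; Joining takes a search result supplied by the caller, and quitting only destroys the session.
; Failed host and join attempts print red bilingual English and Chinese error messages.
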(event `HostGameEvent`
  (`CreateSessionCallbackProxy.CreateSession` (`GameplayStatics.GetPlayerController` 0) 10 true
    (:`OnSuccess`
      (`GameplayStatics.OpenLevel` "WestTown" true "listen"))
    (:`OnFailure`
      (`KismetSystemLibrary.PrintString` "Create room error!創建房間失敗!" true true (struct :`R` 1.0 :`A` 1.0)))))

(event `QuitGameEvent`
  (`DestroySessionCallbackProxy.DestroySession` (`GameplayStatics.GetPlayerController` 0)))

(event `JoinGameEvent`
  (params (SearchResult :type "BlueprintSessionResult Structure"))
  (`JoinSessionCallbackProxy.JoinSession` (`GameplayStatics.GetPlayerController` 0) SearchResult
    (:`OnFailure`
      (`KismetSystemLibrary.PrintString` "Join in session failed.聯機失敗." true true (struct :`R` 1.0 :`A` 1.0)))))