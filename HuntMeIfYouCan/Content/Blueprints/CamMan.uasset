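; CamMan is a pawn, apparently a camera, that automatically yaws its controller every frame.
; Tick feeds Rotation into controller yaw input and accumulates it in TotalRotation.
; When the total passes a symmetric limit on either side, an unnamed operation modifies Rotation, likely reversing it for a back-and-forth pan.
; The step is applied per frame without delta time, so pan speed depends on frame rate.
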(event `self.ReceiveTick`
  (params (DeltaSeconds :type "Float (single-precision)"))
  (bind _rotation (`self.Rotation`))
  (`self.AddControllerYawInput` _rotation)
  (bind _output_get (set `self.TotalRotation` (+ _rotation (`self.TotalRotation`))))
  (if (> _output_get 15.0)
    (`/Engine/EditorBlueprintResources/StandardMacros.NegateFloat` (`self.Rotation`))
    (elif (<= _output_get -15.0)
      (`/Engine/EditorBlueprintResources/StandardMacros.NegateFloat` (`self.Rotation`)))))

(event `self.ReceiveBeginPlay`)

(event `self.ReceiveActorBeginOverlap`
  (params (OtherActor :type "Actor Object Reference")))

(fn `UserConstructionScript`)