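; BP_HMIYCGameMode is a game mode that spawns a BP_Civilian pawn for each player who logs in.
; On authority, PostLogin calls ClientPostLogin, which fills a cached array of PlayerStart actors when it is empty.
; It calls DestroyActor on the new PlayerController, then spawns the civilian at a random cached start, has that same controller possess it and sets game-only input.
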(event `self.ReceiveBeginPlay`)

(event `self.ReceiveTick`
  (params (DeltaSeconds :type "Float (single-precision)")))

(event `self.K2_PostLogin`
  (params (NewPlayer :type "PlayerController Object Reference"))
  (`/Engine/EditorBlueprintResources/ActorMacros.Switch Has Authority`
    (:`Authority`
      (`self.ClientPostLogin` NewPlayer))))

(fn `ClientPostLogin`
  (params (NewPlayer :type "PlayerController Object Reference"))
  (bind _playerstartpostion (`self.PlayerStartPostion`))
  (bind _returnvalue (`KismetArrayLibrary.Array_Length` _playerstartpostion))
  (if (== _returnvalue 0)
    (bind _outactors (`GameplayStatics.GetAllActorsOfClass` "/Script/Engine.PlayerStart"))
    (for _array_element _outactors
      (`KismetArrayLibrary.Array_Add` (`self.PlayerStartPostion`) _array_element)))
  (`self.K2_DestroyActor` NewPlayer)
  (bind _returnvalue_2 (`|SpawnActorFromClass` "/Game/Blueprints/BP_Civilian.BP_Civilian_C" (`self.GetTransform` (`KismetArrayLibrary.Array_Get` _playerstartpostion (`KismetMathLibrary.RandomIntegerInRange` 0 (- _returnvalue 1))))))
  (`Controller.Possess` NewPlayer _returnvalue_2)
  (`WidgetBlueprintLibrary.SetInputMode_GameOnly` NewPlayer))

(fn `UserConstructionScript`)